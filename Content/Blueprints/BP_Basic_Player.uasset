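; BP_Basic_Player is a basic player character with movement, jumping and mouse look.
; Forward/back and right/left axis inputs drive movement input along the actor's forward and right vectors.
; Look axes feed controller yaw and pitch directly, and the Jump action calls the built-in Jump on press.
; All logic sits in the Event Graph, and the construction script is empty.
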(event Input|ActionEvents|InputActionJump
  (params (Key :type Key%20Structure :default "None"))
  ;[0.581 0.5395 1] Movement Jump
  (:Pressed
    (Character|Jump)))

(event Input|AxisEvents|InputAxisForwards/Backwards
  (params (AxisValue :type Float%20%28single-precision%29))
  ;[0.5213 0.4875 1] Movement Forward/Back/Right/Left
  (Pawn|Input|AddMovementInput (Transformation|GetActorForwardVector) AxisValue false))

(event Input|AxisEvents|InputAxisRight/Left
  (params (AxisValue :type Float%20%28single-precision%29))
  ;[0.5213 0.4875 1] Movement Forward/Back/Right/Left
  (Pawn|Input|AddMovementInput (Transformation|GetActorRightVector) AxisValue false))

(event Input|AxisEvents|InputAxisLookLeft/Right
  (params (AxisValue :type Float%20%28single-precision%29))
  ;[1 0.4137 0.3998] Mouse Look Right/Left
  (Pawn|Input|AddControllerYawInput AxisValue))

(event Input|AxisEvents|InputAxisLookUp/Down
  (params (AxisValue :type Float%20%28single-precision%29))
  ;[1 0.4137 0.3998] Mouse Look Right/Left
  (Pawn|Input|AddControllerPitchInput AxisValue))

(fn ConstructionScript)